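; BP_Apple is an edible apple pickup that moves along a path and is consumed on overlap.
; On BeginPlay, a Timeline drives the mesh's world location by lerping between the SceneBottom and SceneTop markers.
; When any actor overlaps the Box, the apple sends it CanEatMessage, plays the AppleBitEvent audio event attached to the mesh, then destroys itself.
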(event OnComponentBeginOverlap(Box)
  (params (OverlappedComponent :type Primitive%20Component%20Object%20Reference) (OtherActor :type Actor%20Object%20Reference) (OtherComp :type Primitive%20Component%20Object%20Reference) (OtherBodyIndex :type Integer) (bFromSweep :type Boolean) (SweepResult :type Hit%20Result%20Structure%20%28by%20ref%29))
  (Class|BPICanEat|CanEat(Message) OtherActor)
  (Class|FMODBlueprintStatics|PlayEventAttached "/Game/FMOD/Events/SFX/AppleBitEvent.AppleBitEvent" (Variables|Default|GetStaticMesh) "None" "0, 0, 0" "KeepRelativeOffset")
  (Actor|DestroyActor))

(event EventBeginPlay
  (bind _alpha (Timeline|Timeline Play)
    (:Update
      (Transformation|SetWorldLocation (Variables|Default|GetStaticMesh) (Math|Vector|Lerp(Vector) (Transformation|GetWorldLocation (Variables|Default|GetSceneBottom)) (Transformation|GetWorldLocation (Variables|Default|GetSceneTop)) _alpha) false false))))

(fn ConstructionScript)